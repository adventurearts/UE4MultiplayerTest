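; Prototype game instance that provides the entry points for hosting and joining multiplayer matches.
; HostGame opens the Arena level as a listen server, and JoinGame passes an IP address to JoinURLGame for a direct connection.
; Disconnected leftover nodes hold unused experiments: LAN session create, find and join with Portuguese debug prints, a HostMatch call, and a hardcoded IP connect.
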(event `Host Game`
  ;[0.5249 1 0.5873] Host Game
  (`GameplayStatics.OpenLevel` "Arena" true "listen"))

(event `Join Game`
  (params (`IP Address` :type String))
  ;[1 0.4478 0.4578] Join Game
  (`self.JoinURLGame` `IP Address`))