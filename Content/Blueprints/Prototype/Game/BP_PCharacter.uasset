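; BP_PCharacter is a prototype player character with basic movement, look, jump and crouch input.
; Axis inputs drive movement along actor forward and right vectors plus controller yaw and pitch.
; Releasing Jump jumps locally and calls ServerJump, which relays through MakeAllJump and MakeJump, setting a button flag that is never cleared.
; Crouch follows press and release directly, leaving MakeCrouch and MakeUnCrouch as empty stubs.
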(event `ServerJump`
  (`self.MakeAllJump`)
  (`self.MakeJump`))

(event `InputAxis|Forward`
  (params (AxisValue :type "Float (single-precision)"))
  ;[0.525 1 0.4583] Movement
  (`self.AddMovementInput` (`self.GetActorForwardVector`) AxisValue))

(event `InputAxis|LookUp`
  (params (AxisValue :type "Float (single-precision)"))
  ;[0.525 1 0.4583] Movement
  (`self.AddControllerPitchInput` AxisValue))

(event `MakeAllJump`
  (`self.MakeJump`))

(event `InputAxis|Turn`
  (params (AxisValue :type "Float (single-precision)"))
  ;[0.525 1 0.4583] Movement
  (`self.AddControllerYawInput` AxisValue))

(event `InputAxis|StrafeRight`
  (params (AxisValue :type "Float (single-precision)"))
  ;[0.525 1 0.4583] Movement
  (`self.AddMovementInput` (`self.GetActorRightVector`) AxisValue))

(event `MakeJump`
  (`self.Jump`)
  (set `self.Jump Button Down` true))

(event `InputAction|Jump`
  (params (Key :type "Key Structure" :default "AnyKey"))
  ;[0.525 1 0.4583] Movement
  (:`Released`
    (`self.MakeJump`)
    (`self.ServerJump`)))

(event `InputAction|Crouch`
  (params (Key :type "Key Structure" :default "AnyKey"))
  ;[0.525 1 0.4583] Movement
  (:`Pressed`
    (`self.Crouch`)
    (set `self.Crouch Button Down` true))
  (:`Released`
    (`self.UnCrouch`)
    (set `self.Crouch Button Down` false)))

(event `MakeCrouch`)

(event `MakeUnCrouch`)

(fn `UserConstructionScript`)